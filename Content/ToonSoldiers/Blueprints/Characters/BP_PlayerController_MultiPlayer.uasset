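; Player controller for ToonSoldiers multiplayer that spawns the player's soldier and drives the gameplay UI.
; On BeginPlay, the local controller checks the GameInstance's game state, then spawns the selected soldier at a random PlayerStart and possesses it.
; Possessing a soldier shows the HUD, which is fetched through the GameInstance.
; P toggles the pause menu, holding Tab shows scores, and DebugPause flips a pause flag and mouse cursor.
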(event Custom|SpawnSoldierEvent
  (params (CustomSoldier :type DS%20Custom%20Soldier%20Structure))
  (bind _outactors (Actor|GetAllActorsOfClass "/Script/Engine.PlayerStart"))
  (bind _returnvalue (Game|SpawnActorfromClass "/Game/ToonSoldiers/Blueprints/Characters/BP_ToonSoldier.BP_ToonSoldier_C" (Transformation|GetActorTransform (.OutItem (Utilities|Array|Random _outactors))) "Undefined" self CustomSoldier 0))
  (Pawn|Possess self _returnvalue))

(event EventBeginPlay
  ;[0.3125 1 0] 生成并控制Pawn
  (if (Pawn|IsLocalPlayerController)
    (bind _asbp_game_instance (Utilities|Casting|CastToBP_GameInstance (Game|GetGameInstance)))
    (if (Utilities|Array|ContainsItem (Utilities|Array|MakeArray "NewEnumerator4" "NewEnumerator5") (Variables|/Game/ToonSoldiers/Blueprints/BP_GameInstance.BP_GameInstance_C|GetGameState _asbp_game_instance))
      (CallFunction|SpawnSoldierEvent (Variables|/Game/ToonSoldiers/Blueprints/BP_GameInstance.BP_GameInstance_C|GetSelectedSoldier _asbp_game_instance)))))

(event EventPossess
  (params (PossessedPawn :type Pawn%20Object%20Reference))
  (Utilities|Casting|CastToBP_ToonSoldier PossessedPawn)
  (CallFunction|ShowGameplayUIEvent))

(event Input|ActionEvents|InputActionDebugPause
  (params (Key :type Key%20Structure :default "None"))
  (:Pressed
    (if (Variables|Default|GetIsPaused)
      (Variables|Default|SetIsPaused false)
      (Variables|Default|SetbShowMouseCursor false)
      (else
        (Variables|Default|SetIsPaused true)
        (Variables|Default|SetbShowMouseCursor true)))))

(event Input|KeyboardEvents|Tab
  (params (Key :type Key%20Structure :default "None"))
  (bind _returnvalue (Game|GetGameInstance))
  (:Pressed
    (bind _asbp_game_instance (Utilities|Casting|CastToBP_GameInstance _returnvalue))
    (Default|TogglePlayerScores (Default|GetGameplayUI _asbp_game_instance)))
  (:Released
    (bind _asbp_game_instance_2 (Utilities|Casting|CastToBP_GameInstance _returnvalue))
    (Default|SwitchtoGameplayHUD (Default|GetGameplayUI _asbp_game_instance_2))))

(event Input|KeyboardEvents|P
  (params (Key :type Key%20Structure :default "None"))
  (:Pressed
    (bind _asbp_game_instance (Utilities|Casting|CastToBP_GameInstance (Game|GetGameInstance)))
    (Utilities|IsValid (Default|GetGameplayUI _asbp_game_instance)
      (:Is%20Valid
        (Default|TogglePauseMenu (Default|GetGameplayUI _asbp_game_instance))))))

(event Custom|ShowGameplayUIEvent
  (Utilities|FlowControl|Sequence
    (:then_0
      (bind _asbp_game_instance (Utilities|Casting|CastToBP_GameInstance (Game|GetGameInstance)))
      (Utilities|IsValid (Default|GetGameplayUI _asbp_game_instance)
        (:Is%20Valid
          (UserInterface|Viewport|AddtoViewport (Default|GetGameplayUI _asbp_game_instance) 0)
          (Default|SwitchtoGameplayHUD (.GameplayUI (CallFunction|GetGameplayUI))))))))

(event Custom|Debug
  (Development|PrintString (Utilities|GetObjectName (Pawn|GetControlledPawn)))
  (Utilities|FlowControl|Delay 1.0)
  (Development|PrintString (Utilities|GetObjectName (Pawn|GetControlledPawn))))

(fn ConstructionScript)

(fn GetGameplayUI
  (if (Pawn|IsLocalPlayerController)
    (bind _asbp_game_instance (Utilities|Casting|CastToBP_GameInstance (Game|GetGameInstance))
      (:then
        (return true (Default|GetGameplayUI _asbp_game_instance)))
      (:CastFailed
        _)))
  (return false 0))