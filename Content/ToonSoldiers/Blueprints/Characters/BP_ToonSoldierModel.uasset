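; Possessable preview model for customizing a toon soldier, loading the GameInstance's selected soldier on possession and rotating on Turn input.
; Head, equipment and legs follow the body mesh through master pose, with functions to swap parts or override material while updating the CustomSoldier struct.
; A scene capture showing only this actor feeds ScreenShot, which exports a timestamped PNG named after the soldier and returns its path.
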(event Custom|SetBody
  (params (Soldier :type DS%20Custom%20Soldier%20Structure))
  (bind (_soldiername _head _body _equipment _legs _overridedmaterial) (Utilities|Struct|BreakDS_CustomSoldier Soldier))
  (Variables|Default|SetCustomSoldier Soldier)
  (Class|SkinnedMeshComponent|SetSkeletalMesh (Variables|Default|GetHead) _head false)
  (Class|SkinnedMeshComponent|SetSkeletalMesh (Variables|Character|GetMesh) _body false)
  (Class|SkinnedMeshComponent|SetSkeletalMesh (Variables|Default|GetEquipment) _equipment false)
  (Class|SkinnedMeshComponent|SetSkeletalMesh (Variables|Default|GetLegs) _legs false)
  (Utilities|IsValid _overridedmaterial
    (:Is%20Valid
      (Rendering|Material|SetMaterial (Variables|Character|GetMesh) 0 _overridedmaterial))))

(event EventTick
  (params (DeltaSeconds :type Float%20%28single-precision%29))
  (bind _output_get (Variables|Default|SetAccumulation (+ DeltaSeconds (Variables|Default|GetAccumulation))))
  (if (> _output_get (Variables|Default|GetNextTimeForAnimation))
    _))

(event EventPossessed
  (params (NewController :type Controller%20Object%20Reference))
  (Class|GameplayStatics|SetViewportMouseCaptureMode "CaptureDuringMouseDown")
  (bind _as玩家控制器 (Utilities|Casting|CastToPlayerController NewController))
  (Variables|/Script/Engine.PlayerController|SetbShowMouseCursor _as玩家控制器 true)
  (bind _asbp_game_instance (Utilities|Casting|CastToBP_GameInstance (Game|GetGameInstance)))
  (CallFunction|SetBody (Variables|/Game/ToonSoldiers/Blueprints/BP_GameInstance.BP_GameInstance_C|GetSelectedSoldier _asbp_game_instance))
  (Development|SetHiddeninGame (Variables|Default|GetWeapon) false false)
  (Components|Activation|Activate (Variables|Default|GetModelCapture) false))

(event Input|AxisEvents|InputAxisTurn
  (params (AxisValue :type Float%20%28single-precision%29))
  (Class|Actor|AddActorWorldRotation (* "0,-4.000000, 0" AxisValue)))

(fn ConstructionScript
  (Utilities|FlowControl|Sequence
    (:then_0
      (Class|SkinnedMeshComponent|SetMasterPoseComponent (Variables|Default|GetEquipment) (Variables|Character|GetMesh) false))
    (:then_1
      (Utilities|Array|Add (Variables|/Script/Engine.SceneCaptureComponent|GetShowOnlyActors (Variables|Default|GetModelCapture)) self))))

(fn SetBodyPart
  (params (BodyPart :type E_BodyPart%20Enum :default "NewEnumerator0") (Mesh :type Skeletal%20Mesh%20Object%20Reference))
  (bind _customsoldier (Variables|Default|GetCustomSoldier))
  (Class|SkinnedMeshComponent|SetSkeletalMesh (Utilities|Select :Index BodyPart :NewEnumerator0 (Variables|Default|GetHead) :NewEnumerator1 (Variables|Character|GetMesh) :NewEnumerator2 (Variables|Default|GetEquipment) :NewEnumerator3 (Variables|Default|GetLegs)) Mesh false)
  (switch Utilities|FlowControl|Switch|SwitchonE_BodyPart BodyPart
    (:NewEnumerator0
      (Utilities|Struct|SetmembersinDS_CustomSoldier _customsoldier Mesh))
    (:NewEnumerator1
      (Utilities|Struct|SetmembersinDS_CustomSoldier _customsoldier Mesh))
    (:NewEnumerator2
      (Utilities|Struct|SetmembersinDS_CustomSoldier _customsoldier Mesh))
    (:NewEnumerator3
      (Utilities|Struct|SetmembersinDS_CustomSoldier _customsoldier Mesh))))

(fn SetMaterial
  (params (Material :type Material%20Interface%20Object%20Reference))
  (Rendering|Material|SetMaterial (Variables|Default|GetHead) 0 Material)
  (Utilities|Struct|SetmembersinDS_CustomSoldier (Variables|Default|GetCustomSoldier) Material))

(fn ScreenShot
  (bind _returnvalue (Math|DateTime|UTCNow))
  (if (Utilities|Array|IsEmpty (.SoldierName (Utilities|Struct|BreakDS_CustomSoldier (Variables|Default|GetCustomSoldier))))
    _
    (else
      (bind _asbp_game_instance (Utilities|Casting|CastToBP_GameInstance (Game|GetGameInstance))
        (:then
          (bind _projectdir (Default|GetProjectSaveDir _asbp_game_instance))
          (bind _output_get (LocalVariables|SetFileName (Utilities|String|Append "Preview_" (.SoldierName (Utilities|Struct|BreakDS_CustomSoldier (Variables|Default|GetCustomSoldier))) "_" (Utilities|String|Append (Utilities|String|ToString(Integer) (Class|KismetMathLibrary|GetYear _returnvalue)) "-" (Utilities|String|ToString(Integer) (Class|KismetMathLibrary|GetMonth _returnvalue)) "-" (Utilities|String|ToString(Integer) (Class|KismetMathLibrary|GetDay _returnvalue)) "-" (Utilities|String|ToString(Integer) (Class|KismetMathLibrary|GetHour _returnvalue)) "-" (Utilities|String|ToString(Integer) (Class|KismetMathLibrary|GetMinute _returnvalue)) "-" (Utilities|String|ToString(Integer) (Class|KismetMathLibrary|GetSecond _returnvalue)) "-" (Utilities|String|ToString(Integer) (Math|DateTime|GetMillisecond _returnvalue))) ".png")))
          ;[1 0.5156 0] 生成截图图片文件
          (Rendering|ExportRenderTarget (Variables|/Script/Engine.SceneCaptureComponent2D|GetTextureTarget (Variables|Default|GetModelCapture)) _projectdir _output_get)
          (return (Utilities|String|Append _projectdir (LocalVariables|GetFileName))))
        (:CastFailed
          _))))
  (return ""))

(fn MakeCustomSoldier
  (bind _customsoldier (Variables|Default|GetCustomSoldier))
  (bind (_soldiername _head _body _equipment _legs _overridedmaterial) (Utilities|Struct|BreakDS_CustomSoldier _customsoldier))
  (return (Utilities|Struct|MakeDS_CustomSoldier _soldiername _head _body _equipment _legs _overridedmaterial)))