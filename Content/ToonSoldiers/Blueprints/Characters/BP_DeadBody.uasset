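; BP_DeadBody is a soldier corpse actor that plays an animation, presumably a death, on a modular body.
; On BeginPlay it applies CustomSoldier's head, body, equipment and leg meshes plus any material override, then plays the animation once on all four parts.
; A timer fires SetRagDoll after the animation's length, but that event is empty.
; SetCustomPhysics assigns physics assets with simulation off but is uncalled here; CustomSoldier's OnRep is empty.
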(event Custom|SetRagDoll)

(event Custom|SetBody
  (bind _customsoldier (Variables|Default|GetCustomSoldier))
  (bind (_soldiername _head _body _equipment _legs _overridedmaterial) (Utilities|Struct|BreakDS_CustomSoldier _customsoldier))
  (Utilities|FlowControl|Sequence
    (:then_0
      (Class|SkinnedMeshComponent|SetSkeletalMesh (Variables|Default|GetHead) _head false)
      (Class|SkinnedMeshComponent|SetSkeletalMesh (Variables|Character|GetMesh) _body false)
      (Class|SkinnedMeshComponent|SetSkeletalMesh (Variables|Default|GetEquipment) _equipment false)
      (Class|SkinnedMeshComponent|SetSkeletalMesh (Variables|Default|GetLegs) _legs false)
      (Utilities|IsValid _overridedmaterial
        (:Is%20Valid
          (Rendering|Material|SetMaterial (Variables|Character|GetMesh) 0 _overridedmaterial))))))

(event Custom|SetCustomPhysics
  (bind _mesh (Variables|Character|GetMesh))
  (bind _legs (Variables|Default|GetLegs))
  (Components|SkinnedMesh|SetPhysicsAsset _mesh "/Game/ToonSoldiers/Assets/Meshes/ToonSoldiers/Characters_PhysicsAsset_Body.Characters_PhysicsAsset_Body" true)
  (Physics|SetSimulatePhysics _mesh false)
  (Components|SkinnedMesh|SetPhysicsAsset _legs "/Game/ToonSoldiers/Assets/Meshes/ToonSoldiers/Characters_PhysicsAsset_Legs.Characters_PhysicsAsset_Legs" true)
  (Physics|SetSimulatePhysics _legs false))

(event EventBeginPlay
  (CallFunction|SetBody)
  (Utilities|Time|SetTimerbyEvent (delegate Custom|SetRagDoll) (Variables|/Script/Engine.AnimSequenceBase|GetSequenceLength (Variables|Default|GetAnimation)))
  (Components|Animation|PlayAnimation (Variables|Character|GetMesh) (Variables|Default|GetAnimation) false))

(event Collision|EventActorBeginOverlap
  (params (OtherActor :type Actor%20Object%20Reference)))

(event EventTick
  (params (DeltaSeconds :type Float%20%28single-precision%29)))

(fn ConstructionScript)

(fn OnRepCustomSoldier)