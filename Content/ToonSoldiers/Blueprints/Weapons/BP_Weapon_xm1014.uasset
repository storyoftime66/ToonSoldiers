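; XM1014 shotgun weapon Blueprint, with server-side timed firing and reloading, and simulated sound, muzzle flash, tracer and holder animation.
; Each shot fires multiple cone-spread line traces, applying point damage per actor scaled by repeat hits; the count starts at zero, so lone pellets deal none.
; A centre trace aims the cosmetic projectile.
; Equipping attaches first/third-person meshes, sets local ammo UI and crosshair, and pre-warms a projectile pool.
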(event EventBeginPlay
  (|CallParentFunction) ; 此节点被禁用，将不会被调用。\n从引脚连出引线来编译功能。
)

(event Collision|EventActorBeginOverlap
  (params (OtherActor :type Actor%20Object%20Reference))
  (|CallParentFunction OtherActor) ; 此节点被禁用，将不会被调用。\n从引脚连出引线来编译功能。
)

(event EventTick
  (params (DeltaSeconds :type Float%20%28single-precision%29))
  (|CallParentFunction DeltaSeconds) ; 此节点被禁用，将不会被调用。\n从引脚连出引线来编译功能。
)

(event Custom|WeaponSimulateImpact
  ;[0.4766 1 0] 射击
)

(event EventWeaponSimulateShooting
  ;[0.4766 1 0] 射击
  (|CGraph_WeaponSimulateShooting))

(event EventServerWeaponHandleShooting
  ;[0.4766 1 0] 射击
  (Networking|SwitchHasAuthority
    (:Authority
      (|CGraph_ServerWeaponHandleShooting))))

(event EventServerWeaponStartShooting
  ;[0.4766 1 0] 射击
  (|CGraph_ServerWeaponStartShooting))

(event EventSimulateonEquipped
  ;[1 0.02344 0] 装备
  (|CGraph_SimulateOnEquipped))

(event EventServerWeaponStopShooting
  ;[0.4766 1 0] 射击
  (Variables|Default|SetBurstCount 0))

(event EventWeaponStopSimulatingShooting
  ;[0.4766 1 0] 射击
  (|CGraph_WeaponStopSimulatingShooting))

(event EventServerWeaponReload
  ;[0.1016 1 0] 装弹
  (|CGraph_ServerWeaponReload))

(event EventWeaponSimulateReloading
  ;[0.1016 1 0] 装弹
  (|CGraph_WeaponSimulateReloading))

(fn ConstructionScript
  (|CallParentFunction))