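; UMP45 weapon Blueprint for a toon soldier shooter, handling equipping, firing and reloading.
; The server runs a retriggerable-delay fire loop, line-tracing within a CrosshairSpread cone to damage Characters, and refills the clip after a delay.
; Simulate events play effects from the last hit, including cosmetic tracers from a pool warmed on equip, and widen the local crosshair spread.
; Equipping attaches first- and third-person meshes, hides one, and sets up local ammo and crosshair UI.
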(event EventBeginPlay)

(event Collision|EventActorBeginOverlap
  (params (OtherActor :type Actor%20Object%20Reference))
  (|CallParentFunction OtherActor) ; 此节点被禁用，将不会被调用。\n从引脚连出引线来编译功能。
)

(event EventTick
  (params (DeltaSeconds :type Float%20%28single-precision%29))
  (if (Variables|Default|GetIsEquipped)
    (|CGraph_UpdateCrosshairSpread)))

(event Custom|WeaponSimulateImpact
  ;[1 0.7031 0] 射击
  (|CGraph_WeaponSimulateImpact))

(event EventServerWeaponReload
  ;[1 0.7734 0] 装弹
  (|CGraph_ServerWeaponReload))

(event EventWeaponSimulateShooting
  ;[1 0.7031 0] 射击
  (|CGraph_WeaponSimulateShooting))

(event EventWeaponStopSimulatingShooting
  ;[1 0.7031 0] 射击
  (|CGraph_WeaponStopSimulatingShooting))

(event EventWeaponSimulateReloading
  ;[1 0.7734 0] 装弹
  (|CGraph_WeaponSimulateReloading))

(event EventServerWeaponHandleShooting
  ;[1 0.7031 0] 射击
  (Networking|SwitchHasAuthority
    (:Authority
      (|CGraph_ServerWeaponHandleShooting))))

(event EventServerWeaponStartShooting
  ;[1 0.7031 0] 射击
  (|CGraph_ServerWeaponStartShooting))

(event EventServerWeaponStopShooting
  ;[1 0.7031 0] 射击
  (Variables|Default|SetBurstCount 0))

(event EventSimulateonEquipped
  ;[0 0.5781 1] 装备
  (|CGraph_SimulateOnEquipped))

(fn ConstructionScript
  (|CallParentFunction))