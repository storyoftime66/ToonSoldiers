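; BP_WeaponBase is the base Blueprint for held weapons, defining shared state, queries and empty events for shooting, reloading and equipping.
; Helpers gate firing by ammo, reload state and fire-mode burst limit, and pick the first- or third-person mesh by whether the holder is locally controlled.
; RepNotifies on holder, burst count, hit result and reloading trigger the simulate events, while ammo updates the local holder's UI.
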(event EventBeginPlay)

(event Collision|EventActorBeginOverlap
  (params (OtherActor :type Actor%20Object%20Reference)))

(event EventTick
  (params (DeltaSeconds :type Float%20%28single-precision%29)))

(event Custom|WeaponSimulateShooting
  ;[1 0.4922 0] 射击
)

(event Custom|ServerWeaponHandleShooting
  ;[1 0.4922 0] 射击
)

(event Custom|ServerWeaponReload
  ;[1 0 0.8672] 装弹
)

(event Custom|WeaponSimulateReloading
  ;[1 0 0.8672] 装弹
)

(event Custom|WeaponStopSimulatingShooting
  ;[1 0.4922 0] 射击
)

(event Custom|ServerWeaponStopShooting
  ;[1 0.4922 0] 射击
)

(event Custom|ServerWeaponStartShooting
  ;[1 0.4922 0] 射击
)

(event Custom|ServerOnEquipped
  (params (NewHolder :type BP%20Toon%20Soldier%20Object%20Reference))
  ;[0.4766 1 0] 拾取和装备
)

(event Custom|SimulateOnEquipped
  ;[0.4766 1 0] 拾取和装备
)

(fn ConstructionScript
  (Variables|武器|武器状态|SetAmmoInClip (Variables|武器|武器属性|GetAmmoPerClip)))

(fn IsHolderLocallyControlled
  (bind _holder (Variables|Default|GetHolder)
    (:then
      (return (Pawn|IsLocallyControlled _holder)))
    (:else
      (return false))))

(fn GetHolderController
  (bind _holder (Variables|Default|GetHolder)
    (:then
      (return (Pawn|GetController _holder)))
    (:else
      (return 0))))

(fn GetMuzzlePoint
  (return (Transformation|GetSocketLocation (select (Holder|IsHolderLocallyControlled) (Variables|Default|GetFirstPersonWeaponMesh) (Variables|Default|GetThirdPersonWeaponMesh)) "Muzzle")))

(fn GetMuzzleTranform
  (return (Transformation|GetSocketTransform (select (Holder|IsHolderLocallyControlled) (Variables|Default|GetFirstPersonWeaponMesh) (Variables|Default|GetThirdPersonWeaponMesh)) "Muzzle" "RTS_World")))

(fn CanWeaponShoot
  (if (and (> (Variables|武器|武器状态|GetAmmoInClip) 0.0) (not (Variables|武器|武器状态|GetIsReloading)))
    (return (< (Variables|武器|武器状态|GetBurstCount) (Utilities|Select :Index (Variables|武器|武器状态|GetFireMode) :NewEnumerator0 1 :NewEnumerator1 3 :NewEnumerator2 10000)))
    (else
      (return false))))

(fn GetHolderAimingPoint
  (return (Variables|/Game/ToonSoldiers/Blueprints/Characters/BP_ToonSoldier.BP_ToonSoldier_C|GetAimingPoint (Variables|Default|GetHolder))))

(fn HolderWantstoShoot
  (bind _holder (Variables|Default|GetHolder)
    (:then
      (return (Variables|/Game/ToonSoldiers/Blueprints/Characters/BP_ToonSoldier.BP_ToonSoldier_C|GetWantsToShoot _holder)))
    (:else
      (return false))))

(fn OnRepHolder
  (CallFunction|SimulateonEquipped))

(fn OnRepBurstCount
  (if (not (> (Variables|武器|武器状态|GetBurstCount) 0))
    (CallFunction|WeaponStopSimulatingShooting)))

(fn OnRepAmmoinClip
  (if (Holder|IsHolderLocallyControlled)
    (bind _gameplayui (Variables|武器|UI|GetGameplayUI)
      (:then
        (Default|UpdateAmmo _gameplayui (Variables|武器|武器状态|GetAmmoInClip) (Variables|武器|武器属性|GetAmmoPerClip)))
      (:else))))

(fn CanWeaponReload
  (return (and (not (Variables|武器|武器状态|GetIsReloading)) (< (Variables|武器|武器状态|GetAmmoInClip) (Variables|武器|武器属性|GetAmmoPerClip)))))

(fn GetWeaponMesh
  (return (select (Holder|IsHolderLocallyControlled) (Variables|Default|GetFirstPersonWeaponMesh) (Variables|Default|GetThirdPersonWeaponMesh))))

(fn OnRepIsReloading
  (if (Variables|武器|武器状态|GetIsReloading)
    (CallFunction|WeaponSimulateReloading)))

(fn OnRepLastHitResult
  (CallFunction|WeaponSimulateShooting))