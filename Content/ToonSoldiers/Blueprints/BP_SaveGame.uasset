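; BP_SaveGame stores a list of custom soldiers, each paired with a preview path, for the ToonSoldiers game.
; It keeps two parallel arrays, inserting new entries at the front so the newest comes first.
; Length is the shorter of the two arrays, which bounds indexed reads that also return a validity flag.
; Resize only trims both arrays, never grows them.
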(fn Resize
  (params (NewSize :type Integer))
  (if (> (CallFunction|GetLength) NewSize)
    (Utilities|Array|Resize (Variables|自定义角色存档|GetSoldiers) NewSize)
    (Utilities|Array|Resize (Variables|自定义角色存档|GetSoldierPreviewPaths) NewSize)))

(fn AddSoldier
  (params (Soldier :type DS%20Custom%20Soldier%20Structure) (Preview :type String))
  (Utilities|Array|Insert (Variables|自定义角色存档|GetSoldiers) Soldier)
  (Utilities|Array|Insert (Variables|自定义角色存档|GetSoldierPreviewPaths) Preview))

(fn Get
  (params (Index :type Integer))
  (if (< Index (CallFunction|GetLength))
    (return true (Utilities|Array|Get(acopy) (Variables|自定义角色存档|GetSoldiers) Index) (Utilities|Array|Get(acopy) (Variables|自定义角色存档|GetSoldierPreviewPaths) Index))
    (else
      (return false "" ""))))

(fn GetLength
  (return (Math|Integer|Min(Integer) (Utilities|Array|Length (Variables|自定义角色存档|GetSoldiers)) (Utilities|Array|Length (Variables|自定义角色存档|GetSoldierPreviewPaths)))))