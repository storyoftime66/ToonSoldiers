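; BP_Projectile_Debug is a pooled projectile variant for debugging.
; It extends the parent's pool begin and end events to switch its ACDebugComponent on and off, toggling both activation and component tick.
; Returning to the pool also prints a "PoolEnd" message.
; BeginPlay, overlap and Tick are unused stubs, and construction defers to the parent.
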(event EventBeginPlay
  (|CallParentFunction) ; 此节点被禁用，将不会被调用。\n从引脚连出引线来编译功能。
)

(event Collision|EventActorBeginOverlap
  (params (OtherActor :type Actor%20Object%20Reference))
  (|CallParentFunction OtherActor) ; 此节点被禁用，将不会被调用。\n从引脚连出引线来编译功能。
)

(event EventTick
  (params (DeltaSeconds :type Float%20%28single-precision%29))
  (|CallParentFunction DeltaSeconds) ; 此节点被禁用，将不会被调用。\n从引脚连出引线来编译功能。
)

(event EventOnPoolEnd
  (bind _ac_debugcomponent (Variables|Default|GetAC_DebugComponent))
  (|CallParentFunction)
  (Components|Activation|Deactivate _ac_debugcomponent)
  (Components|Tick|SetComponentTickEnabled _ac_debugcomponent false)
  (Development|PrintString "PoolEnd"))

(event EventOnPoolBegin
  (bind _ac_debugcomponent (Variables|Default|GetAC_DebugComponent))
  (|CallParentFunction)
  (Components|Activation|Activate _ac_debugcomponent true)
  (Components|Tick|SetComponentTickEnabled _ac_debugcomponent true))

(fn ConstructionScript
  (|CallParentFunction))