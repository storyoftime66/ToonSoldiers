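; Pooled rifle tracer projectile that shows a particle effect flying forward from a weapon's shot.
; When taken from the pool it activates its particles and sets velocity along its forward vector.
; It sets its lifespan from the owning weapon's last hit distance, or weapon range if nothing blocked, divided by speed, so the tracer ends at the hit point.
; Returning to the pool deactivates the particles.
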(event EventBeginPlay)

(event Collision|EventActorBeginOverlap
  (params (OtherActor :type Actor%20Object%20Reference)))

(event EventTick
  (params (DeltaSeconds :type Float%20%28single-precision%29)))

(event EventOnPoolEnd
  (|CallParentFunction)
  (Components|Activation|Deactivate (Variables|Default|GetParticleSystem)))

(event EventOnPoolBegin
  (Utilities|FlowControl|Sequence
    (:then_0
      (Components|Activation|Activate (Variables|Default|GetParticleSystem) true)
      (Variables|/Script/Engine.MovementComponent|SetVelocity (Variables|Default|GetProjectileMovement) (* (Transformation|GetActorForwardVector) (Variables|Default|GetProjectileVelocity))))
    (:then_1
      (bind _asbp_weapon_base (Utilities|Casting|CastToBP_WeaponBase (Components|GetOwner)))
      (Variables|Default|SetProjectileLifeSpan (/ (select (.bBlockingHit (Collision|BreakHitResult (Variables|/Game/ToonSoldiers/Blueprints/Weapons/BP_WeaponBase.BP_WeaponBase_C|GetLastHitResult _asbp_weapon_base))) (.Distance (Collision|BreakHitResult (Variables|/Game/ToonSoldiers/Blueprints/Weapons/BP_WeaponBase.BP_WeaponBase_C|GetLastHitResult _asbp_weapon_base))) (Variables|/Game/ToonSoldiers/Blueprints/Weapons/BP_WeaponBase.BP_WeaponBase_C|GetRange _asbp_weapon_base)) (Variables|Default|GetProjectileVelocity))))
    (:then_2
      (|CallParentFunction))))

(fn ConstructionScript)