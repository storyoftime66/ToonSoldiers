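; BP_Projectile_ShotgunTracer is a pooled shotgun tracer projectile that shows a shot's path with a particle effect.
; When taken from the pool, it activates the particle system with a random roll and launches along its forward vector.
; Its lifespan comes from the owning weapon's last hit distance, or range if nothing blocked, divided by projectile velocity.
; Returning to the pool deactivates the particles.
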(event EventBeginPlay
  (|CallParentFunction) ; 此节点被禁用，将不会被调用。\n从引脚连出引线来编译功能。
)

(event Collision|EventActorBeginOverlap
  (params (OtherActor :type Actor%20Object%20Reference))
  (|CallParentFunction OtherActor) ; 此节点被禁用，将不会被调用。\n从引脚连出引线来编译功能。
)

(event EventTick
  (params (DeltaSeconds :type Float%20%28single-precision%29))
  (|CallParentFunction DeltaSeconds) ; 此节点被禁用，将不会被调用。\n从引脚连出引线来编译功能。
)

(event EventOnPoolEnd
  (|CallParentFunction)
  (Components|Activation|Deactivate (Variables|Default|GetParticleSystem)))

(event EventOnPoolBegin
  (bind _particlesystem (Variables|Default|GetParticleSystem))
  (Utilities|FlowControl|Sequence
    (:then_0
      (Components|Activation|Activate _particlesystem true)
      (Transformation|AddRelativeRotation _particlesystem (Math|Rotator|MakeRotator (Math|Random|RandomFloatinRange -1.8e+02 1.8e+02) 0.0 0.0) false false)
      (Variables|/Script/Engine.MovementComponent|SetVelocity (Variables|Default|GetProjectileMovement) (* (Transformation|GetActorForwardVector) (Variables|Default|GetProjectileVelocity))))
    (:then_1
      (bind _asbp_weapon_base (Utilities|Casting|CastToBP_WeaponBase (Components|GetOwner)))
      (Variables|Default|SetProjectileLifeSpan (/ (select (.bBlockingHit (Collision|BreakHitResult (Variables|/Game/ToonSoldiers/Blueprints/Weapons/BP_WeaponBase.BP_WeaponBase_C|GetLastHitResult _asbp_weapon_base))) (.Distance (Collision|BreakHitResult (Variables|/Game/ToonSoldiers/Blueprints/Weapons/BP_WeaponBase.BP_WeaponBase_C|GetLastHitResult _asbp_weapon_base))) (Variables|/Game/ToonSoldiers/Blueprints/Weapons/BP_WeaponBase.BP_WeaponBase_C|GetRange _asbp_weapon_base)) (Variables|Default|GetProjectileVelocity))))
    (:then_2
      (|CallParentFunction))))

(fn ConstructionScript
  (|CallParentFunction))