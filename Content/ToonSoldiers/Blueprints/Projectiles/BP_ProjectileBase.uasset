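; BP_ProjectileBase is a base projectile Blueprint that is reused through an actor pool.
; OnPoolBegin enables collision, visibility, ticking and ProjectileMovement, then starts a one-shot timer when ProjectileLifeSpan is positive.
; The timer fires RecycleActor, which calls ReleaseActor instead of destroying the projectile.
; OnPoolEnd turns collision, visibility, ticking and movement off; no hit or damage logic is defined here.
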(event Custom|RecycleActor
  ;[0.8047 1 0] 生命周期
  (Class|PoolManagerBPLibrary|ReleaseActor))

(event EventBeginPlay)

(event Collision|EventActorBeginOverlap
  (params (OtherActor :type Actor%20Object%20Reference)))

(event EventTick
  (params (DeltaSeconds :type Float%20%28single-precision%29)))

(event EventOnPoolEnd
  (bind _projectilemovement (Variables|Default|GetProjectileMovement))
  (Collision|SetActorEnableCollision false)
  (Rendering|SetActorHiddenInGame true)
  (Actor|Tick|SetActorTickEnabled false)
  (Components|Activation|Deactivate _projectilemovement)
  (Components|Tick|SetComponentTickEnabled _projectilemovement false))

(event EventOnPoolBegin
  (bind _projectilemovement (Variables|Default|GetProjectileMovement))
  (Utilities|FlowControl|Sequence
    (:then_0
      (Collision|SetActorEnableCollision true)
      (Rendering|SetActorHiddenInGame false)
      (Actor|Tick|SetActorTickEnabled true)
      (Components|Activation|Activate _projectilemovement true)
      (Components|Tick|SetComponentTickEnabled _projectilemovement true))
    (:then_1
      ;[0.8047 1 0] 生命周期
      (if (> (Variables|发射物|通用|GetProjectileLifeSpan) 0.0)
        (Utilities|Time|SetTimerbyEvent (delegate Custom|RecycleActor) (Variables|发射物|通用|GetProjectileLifeSpan))))))

(fn ConstructionScript)